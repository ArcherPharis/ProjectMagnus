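; GA_BP_Skittish is a gameplay ability for Irwin's class skills that gives the owning player character a movement speed boost.
; On activation it sets the character's MaxWalkSpeed to a fixed value and spawns a thunder-hit particle at its location, skipping both if that speed is already set.
; The ability ends immediately either way, and nothing in it restores the original speed.
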(event `self.K2_ActivateAbility`
  (bind _returnvalue_owneractor (break `GameplayAbilityActorInfo` (`self.GetActorInfo`)))
  (bind _asplayer_character (cast `PlayerCharacter` _returnvalue_owneractor))
  (bind _charactermovement (`Character.CharacterMovement` _asplayer_character))
  (if (== (`CharacterMovementComponent.MaxWalkSpeed` _charactermovement) 900.0)
    (`self.K2_EndAbility`)
    (else
      (set `CharacterMovementComponent.MaxWalkSpeed` 900.0 _charactermovement)
      (`GameplayStatics.SpawnEmitterAtLocation` "/Game/FXVarietyPack/Particles/P_ky_ThunderBallHit.P_ky_ThunderBallHit" (`Actor.K2_GetActorLocation` _asplayer_character))
      (`self.K2_EndAbility`))))