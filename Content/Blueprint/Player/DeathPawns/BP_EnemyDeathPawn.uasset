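; BP_EnemyDeathPawn is a death pawn in the player Blueprints that plays an overhead camera sequence.
; On BeginPlay it deactivates DeathAboveCam, waits briefly, then reactivates it and records its world location.
; A timeline then lerps the camera straight up from that location, producing a rising view from above.
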(event `self.ReceiveBeginPlay`
  (`ActorComponent.SetActive` (`self.DeathAboveCam`) false false)
  (`KismetSystemLibrary.Delay` 2.0)
  (`ActorComponent.SetActive` (`self.DeathAboveCam`) true false)
  (set `self.start loc` (`SceneComponent.K2_GetComponentLocation` (`self.DeathAboveCam`)))
  (bind (_direction _lfs) (`Timeline|Timeline_0` :!via `PlayFromStart`)
    (:`Update`
      (`SceneComponent.K2_SetWorldLocation` (`self.DeathAboveCam`) (`KismetMathLibrary.VLerp` (`self.start loc`) (+ (`self.start loc`) (0.0 0.0 250.0)) _lfs) false false))))

(fn `UserConstructionScript`)