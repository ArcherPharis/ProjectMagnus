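; BP_DevPlayer2 is a player character Blueprint with a hold-to-aim over-the-shoulder camera.
; Holding right mouse switches rotation from movement-facing to controller yaw, and releasing it switches back.
; Separate Aim and UnAim timelines lerp the spring arm socket offset between centered and shoulder positions.
; It also hides the mesh's weapon bone on BeginPlay and applies damage to itself when G is pressed.
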(event `self.ReceiveBeginPlay`
  (`SkinnedMeshComponent.HideBoneByName` (`self.Mesh`) "weapon" "PBO_None"))

(event `self.ReceiveTick`
  (params (DeltaSeconds :type "Float (single-precision)")))

(event `Key|RightMouseButton`
  (params (Key :type "Key Structure"))
  (bind _returnvalue (`self.GetSpringArm`))
  (bind _charactermovement (`self.CharacterMovement`))
  (:`Pressed`
    (set `self.bUseControllerRotationYaw` true)
    (set `CharacterMovementComponent.bOrientRotationToMovement` false _charactermovement)
    (bind (_direction _y_socket) (`Timeline|Aim` :!via `PlayFromStart`)
      (:`Update`
        (set `SpringArmComponent.SocketOffset` (`KismetMathLibrary.VLerp` (0.0 0.0 75.0) (50.0 50.0 75.0) _y_socket) _returnvalue))))
  (:`Released`
    (set `self.bUseControllerRotationYaw` false)
    (set `CharacterMovementComponent.bOrientRotationToMovement` true _charactermovement)
    (bind (_direction_2 _y_socket_2) (`Timeline|UnAim` :!via `PlayFromStart`)
      (:`Update`
        (set `SpringArmComponent.SocketOffset` (`KismetMathLibrary.VLerp` (0.0 0.0 75.0) (50.0 50.0 75.0) _y_socket_2) _returnvalue)))))

(event `Key|G`
  (params (Key :type "Key Structure"))
  (:`Pressed`
    (`GameplayStatics.ApplyDamage` self 10.0)))

(fn `UserConstructionScript`)