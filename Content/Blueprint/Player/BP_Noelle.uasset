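; Player character Blueprint for Noelle, handling aim movement, camera shifts and death.
; Right mouse or aim events switch between movement-oriented and controller-yaw rotation while timelines blend the spring arm to and from an over-the-shoulder offset.
; Weapon attack state gates the mouse toggle and post-fire un-aim.
; It also hides the mesh's weapon bone, clears stamina-drain effects on stopping, and shows a paused lose screen after death.
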(event `self.ReceiveBeginPlay`
  (`SkinnedMeshComponent.HideBoneByName` (`self.Mesh`) "weapon" "PBO_None"))

(event `self.ReceiveTick`
  (params (DeltaSeconds :type "Float (single-precision)")))

(event `self.BeginAimMovement`
  (set `self.bUseControllerRotationYaw` true :!label _label)
  (set `CharacterMovementComponent.bOrientRotationToMovement` false (`self.CharacterMovement`))
  (bind (_direction _y_socket) (`Timeline|Aim` :!via `PlayFromStart`)
    (:`Update`
      (set `SpringArmComponent.SocketOffset` (`KismetMathLibrary.VLerp` (0.0 0.0 75.0) (50.0 50.0 75.0) _y_socket) (`self.GetSpringArm`)))))

(event `Key|RightMouseButton`
  (params (Key :type "Key Structure"))
  (bind _returnvalue (`Weapon.GetInAttackEvent` (`self.GetCurrentWeapon`)))
  (:`Pressed`
    (if (not _returnvalue)
      (goto _label)))
  (:`Released`
    (if (not _returnvalue) :!label _label_2
      (`self.SetIsAiming` false :!label _label_3)
      (set `self.bUseControllerRotationYaw` false)
      (set `CharacterMovementComponent.bOrientRotationToMovement` true (`self.CharacterMovement`))
      (bind (_direction _y_socket) (`Timeline|UnAim` :!via `PlayFromStart`)
        (:`Update`
          (set `SpringArmComponent.SocketOffset` (`KismetMathLibrary.VLerp` (0.0 0.0 75.0) (50.0 50.0 75.0) _y_socket) (`self.GetSpringArm`)))))))

(event `self.PostFireEventEffects`
  (goto _label_2))

(event `self.StopAimMovement`
  (goto _label_3))

(event `self.OnStopMoving`
  (`AbilitySystemComponent.RemoveActiveEffectsWithTags` (`AbilitySystemBlueprintLibrary.GetAbilitySystemComponent` self) (struct :`GameplayTags` (struct :`(TagName` "Effect.StaminaDrain")))))

(event `self.DeathEvent`
  (bind _returnvalue (`GameplayStatics.GetPlayerController` 0))
  (`KismetSystemLibrary.Delay` 3.0)
  (`GameplayStatics.SetGamePaused` true)
  (bind _returnvalue_2 (`|CreateWidget` "/Game/UI/ResultScreens/WBP_YouLose.WBP_YouLose_C" _returnvalue))
  (`UserWidget.AddToViewport` _returnvalue_2 0)
  (`WidgetBlueprintLibrary.SetInputMode_UIOnlyEx` _returnvalue null)
  (set `PlayerController.bShowMouseCursor` true _returnvalue))

(fn `UserConstructionScript`)