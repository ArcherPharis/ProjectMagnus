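; BP_ARX2 is a weapon Blueprint that adds camera shake and recoil to the player's aim when attacking.
; OnAttack starts the shake and plays the Recoil timeline, whose pitch and yaw values feed the player controller's look input each update.
; OnStopAttack reverses the timeline at a faster rate, and negatively scaled input during reverse playback pulls the aim back.
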(event `self.ReceiveTick`
  (params (DeltaSeconds :type "Float (single-precision)")))

(event `self.OnAttack`
  (`PlayerController.ClientStartCameraShake` :`self` (`GameplayStatics.GetPlayerController` 0) :`Shake` "/Game/Blueprint/CameraShake/BP_DevGunShake.BP_DevGunShake_C")
  (`TimelineComponent.SetPlayRate` (`self.Recoil`) 1.0)
  (bind (_direction _pitch _yaw) (`Timeline|Recoil` :!via `PlayFromStart` :!label _label)
    (:`Update`
      (switch `ETimelineDirection` _direction
        (:`Forward`
          (`self.UpdatePitchAndInput` _pitch _yaw))
        (:`Backward`
          (`self.UpdatePitchAndInput` (* _pitch -2.5) (* _yaw -2.5)))))))

(event `self.OnStopAttack`
  (`TimelineComponent.SetPlayRate` (`self.Recoil`) 2.5)
  (goto _label :!via `Reverse`))

(fn `UpdatePitchAndInput`
  (params (Pitch :type "Float (single-precision)") (Yaw :type "Float (single-precision)"))
  (bind _returnvalue (`GameplayStatics.GetPlayerController` 0))
  (`PlayerController.AddPitchInput` _returnvalue Pitch)
  (`PlayerController.AddYawInput` _returnvalue Yaw))

(fn `UserConstructionScript`)