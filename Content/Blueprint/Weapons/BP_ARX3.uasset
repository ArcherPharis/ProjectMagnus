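; BP_ARX3 is a weapon Blueprint that handles recoil, camera feedback, impact effects and view rotation for the ARX3.
; Attacking starts a camera shake and a Recoil timeline that feeds pitch and yaw into player 0's controller input.
; Stopping reverses that timeline faster, applying scaled-down opposite input.
; Impacts spawn a Gun_Hit effect, and RotateCharacter uses a timeline to lerp control rotation toward a hit target.
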(event `self.OnAttack`
  (`PlayerController.ClientStartCameraShake` :`self` (`GameplayStatics.GetPlayerController` 0) :`Shake` "/Game/Blueprint/CameraShake/BP_DevGunShake.BP_DevGunShake_C")
  (`TimelineComponent.SetPlayRate` (`self.Recoil`) 1.0)
  (bind (_direction _pitch _yaw) (`Timeline|Recoil` :!via `PlayFromStart` :!label _label)
    (:`Update`
      (switch `ETimelineDirection` _direction
        (:`Forward`
          (`self.UpdatePitchAndInput` _pitch _yaw))
        (:`Backward`
          (`self.UpdatePitchAndInput` (* _pitch -0.1) (* _yaw -0.1)))))))

(event `self.ReceiveTick`
  (params (DeltaSeconds :type "Float (single-precision)")))

(event `self.OnStopAttack`
  (`TimelineComponent.SetPlayRate` (`self.Recoil`) 2.5)
  (goto _label :!via `Reverse`))

(event `self.SpawnImpactEffects`
  (params (result :type "HitResult Structure"))
  (`NiagaraFunctionLibrary.SpawnSystemAtLocation` "/Game/VFX/Gun_Hit.Gun_Hit" result_ImpactPoint))

(event `self.RotateCharacter`
  (params (character :type "Character_Base Object Reference") (result :type "Actor Object Reference"))
  (bind _returnvalue (`GameplayStatics.GetPlayerCameraManager` 0))
  (bind (_direction _alpha) (`Timeline|rotate` :!via `PlayFromStart`)
    (:`Update`
      (`Controller.SetControlRotation` (`Pawn.GetController` character) (`KismetMathLibrary.RLerp` (`self.K2_GetActorRotation` _returnvalue) (`KismetMathLibrary.FindLookAtRotation` (`self.K2_GetActorLocation` _returnvalue) (`self.K2_GetActorLocation` result)) _alpha)))))

(fn `UpdatePitchAndInput`
  (params (Pitch :type "Float (single-precision)") (Yaw :type "Float (single-precision)"))
  (bind _returnvalue (`GameplayStatics.GetPlayerController` 0))
  (`PlayerController.AddPitchInput` _returnvalue Pitch)
  (`PlayerController.AddYawInput` _returnvalue Yaw))

(fn `UserConstructionScript`)